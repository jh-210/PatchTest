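; Game mode that starts the game's content patching at play start and reports its download and mount progress on screen.
; BeginPlay calls PatchGame on BP_MyGameInstance and, on failure, has a counter-gated delayed retry whose result is not stored.
; While patching is flagged in progress, Tick prints both loading percentages and whether both have reached completion, as debug strings.
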(event EventBeginPlay
  (bind _asbp_my_game_instance (Utilities|Casting|CastToBP_MyGameInstance (Game|GetGameInstance)))
  (bind _output_get (Variables|Default|SetAs%20BP%20My%20Game%20Instance _asbp_my_game_instance))
  (bind _returnvalue (Class|MyGameInstance|PatchGame _output_get))
  (Variables|Default|SetIs%20Patching%20Is%20Progress _returnvalue)
  (if (not (Variables|Default|GetIs%20Patching%20Is%20Progress))
    (bind _result (Math|Integer|IncrementInt (Variables|Default|GetTry%20Patch%20Count))
      (:%20%20
        (if (not (> _result 0))
          (Utilities|FlowControl|Delay 0.2)
          (Class|MyGameInstance|PatchGame (Variables|Default|GetAs%20BP%20My%20Game%20Instance)))))))

(event EventTick
  (params (DeltaSeconds :type Float%20%28single-precision%29))
  (bind _as_bp_my_game_instance (Variables|Default|GetAs%20BP%20My%20Game%20Instance))
  (bind (_bytesdownloaded _totalbytestodownload _downloadpercent _chunksmounted _totalchunkstomount _mountpercent) (Class|MyGameInstance|GetLoadingProgress _as_bp_my_game_instance))
  (if (Variables|Default|GetIs%20Patching%20Is%20Progress)
    (Development|PrintString (Class|KismetStringLibrary|BuildStringDouble "" "" _downloadpercent "%"))
    (Development|PrintString (Class|KismetStringLibrary|BuildStringDouble "" "" _mountpercent "%"))
    (if (and (>= _downloadpercent 1e+02) (>= _mountpercent 1e+02))
      (Development|PrintString "True")
      (else
        (Development|PrintString "False")))))

(fn ConstructionScript)