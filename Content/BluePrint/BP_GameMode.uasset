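; BP_GameMode is a game mode that starts game content patching through MyGameInstance and reports its progress.
; BeginPlay casts and caches the game instance, then calls PatchGame, retrying after short delays up to a capped count if it returns false.
; While patching is flagged in progress, Tick prints download and mount progress as debug strings, plus a placeholder success or fail message; the flag is never cleared here.
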(event EventBeginPlay
  (bind _asmy_game_instance (Utilities|Casting|CastToMyGameInstance (Game|GetGameInstance))
    (:then
      (bind _output_get (Variables|Default|SetAs%20My%20Game%20Instance _asmy_game_instance))
      (bind _returnvalue (Class|MyGameInstance|PatchGame _output_get :!label _label))
      (bind _output_get_2 (Variables|Default|SetIs%20Patching%20in%20Progress _returnvalue))
      (if (not _output_get_2)
        (bind _result (Math|Integer|IncrementInt (Variables|Default|GetTry%20Patch%20Count))
          (:%20%20
            (if (not (> _result 3))
              (Utilities|FlowControl|Delay 0.2)
              (goto _label))))))
    (:CastFailed
      (Development|PrintString "Cast Fail"))))

(event EventTick
  (params (DeltaSeconds :type Float%20%28single-precision%29))
  (bind _as_my_game_instance (Variables|Default|GetAs%20My%20Game%20Instance))
  (bind (_bytesdownloaded _totalbytestodownload _downloadpercent _chunksmounted _totalchunkstomount _mountpercent) (Class|MyGameInstance|GetLoadingProgress _as_my_game_instance))
  (if (Variables|Default|GetIs%20Patching%20in%20Progress)
    (Development|PrintString (Class|KismetStringLibrary|BuildStringDouble "" "Current Loading Progress : " _downloadpercent "%"))
    (Development|PrintString (Class|KismetStringLibrary|BuildStringDouble "" "Current Mounting Progress : " _mountpercent "%"))
    (if (and (>= _downloadpercent 1.0) (>= _mountpercent 1.0))
      (Development|PrintString "Hello")
      (else
        (Development|PrintString "Fail")))))

(fn ConstructionScript)